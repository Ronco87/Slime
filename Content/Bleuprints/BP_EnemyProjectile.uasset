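; BP_EnemyProjectile is a projectile actor that damages any BP_Slime it hits, despite its enemy naming.
; Its sphere ignores the instigator, and on a slime hit it grants energy to a slime instigator before destroying itself.
; Other hits destroy it immediately, but a slime hit with a non-slime instigator leaves it alive.
; The construction script takes mesh and scale from AmmoData when valid.
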(event `self.ReceiveBeginPlay`
  (`PrimitiveComponent.IgnoreActorWhenMoving` (`self.Sphere`) (`self.GetInstigator`) true))

(event `self.Sphere.OnComponentHit`
  (params (HitComponent :type "PrimitiveComponent Object Reference") (OtherActor :type "Actor Object Reference") (OtherComp :type "PrimitiveComponent Object Reference") (NormalImpulse :type "Vector Structure") (Hit :type "HitResult Structure (by ref)"))
  (cast `/Game/ThirdPerson/Blueprints/BP_Slime` OtherActor
    (:`then`
      (`GameplayStatics.ApplyDamage` OtherActor (`self.Damage`) null self)
      (bind _asbp_slime (cast `/Game/ThirdPerson/Blueprints/BP_Slime` (`self.GetInstigator`)))
      (`/Game/ThirdPerson/Blueprints/BP_Slime.AddEnergy` _asbp_slime 3.0))
    (:`CastFailed`
      _))
  (`self.K2_DestroyActor`))

(fn `UserConstructionScript`
  (bind _sphere1 (`self.Sphere1`))
  (bind _ammodata (`self.AmmoData`))
  (`/Engine/EditorBlueprintResources/StandardMacros.IsValid` _ammodata
    (:`Is Valid`
      (`StaticMeshComponent.SetStaticMesh` _sphere1 (`/Game/Bleuprints/DATAS/PDA_AbsotbableData.Mesh` _ammodata))
      (`SceneComponent.SetRelativeScale3D` _sphere1 (`/Game/Bleuprints/DATAS/PDA_AbsotbableData.MeshScale` _ammodata))
      (`PrimitiveComponent.SetMaterial` (`self.Sphere1`) 0 (`PrimitiveComponent.GetMaterial` _sphere1 0)))))