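; Wave spawner actor that populates the level with BP_Enemy and spawns BP_Boss once the final wave is cleared.
; A looping timer spawns enemies up to the wave quota and live cap, at random reachable navmesh points checked for player distance.
; Each enemy gets random EnemyData, with weighted heavy types in later waves.
; Waves grow in size, update the BP_Slime player's HUD, and restart after a delay once all enemies are gone.
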(event `SpawnEnemy`
  (bind (_randomlocation _returnvalue) (`NavigationSystemV1.K2_GetRandomReachablePointInRadius` (`self.K2_GetActorLocation`) (`self.SpawnRadius`) null null))
  (bind _outactors (`GameplayStatics.GetAllActorsOfClass` "/Game/Bleuprints/BP_Enemy.BP_Enemy_C"))
  (if (< (`KismetArrayLibrary.Array_Length` _outactors) (`self.MaxEnemies`))
    (if _returnvalue
      (if (> (`KismetMathLibrary.VSize` (- _randomlocation (`self.K2_GetActorLocation` (`GameplayStatics.GetPlayerCharacter` 0)))) (`self.MinDistanceToPlayer`))
        (`|SpawnActorFromClass` "/Game/Bleuprints/BP_Enemy.BP_Enemy_C" (`KismetMathLibrary.MakeTransform` (+ _randomlocation (0.0 0.0 100.0))) "AdjustIfPossibleButAlwaysSpawn" "MultiplyWithRoot" null (cast `/Game/Bleuprints/DATAS/PDA_EnemyData` (`KismetMathLibrary.SelectObject` (`self.HeavyType`) (`KismetArrayLibrary.Array_Random` (`self.EnemyTypes`)) (and (>= (`self.Wave`) 4) (`KismetMathLibrary.RandomBoolWithWeight` 0.3))) :!pure true) null)
        (set `self.EnemiesSpawned` (+ (`self.EnemiesSpawned`) 1))))))

(event `StartWave`
  (bind _output_get (set `self.Wave` (+ (`self.Wave`) 1)))
  (set `self.EnemiesToSpawn` (+ _output_get (* (- (`self.Wave`) 1) (`self.EnemiesPerWave`))))
  (set `self.EnemiesSpawned` 0)
  (set `self.bWaveActive` true)
  (`KismetSystemLibrary.PrintString` (`KismetStringLibrary.Concat_StrStr` "Oleada " (`KismetStringLibrary.Conv_IntToString` (`self.Wave`))))
  (bind _asbp_slime (cast `/Game/ThirdPerson/Blueprints/BP_Slime` (`GameplayStatics.GetPlayerCharacter` 0)))
  (bind _hudref (`/Game/ThirdPerson/Blueprints/BP_Slime.HUDRef` _asbp_slime))
  (`/Engine/EditorBlueprintResources/StandardMacros.IsValid` _hudref
    (:`Is Valid`
      (`/Game/Widgets/WBP_HUD.UpdateWave` _hudref (`self.Wave`) (`self.WaveToWin`)))))

(event `WaveTick`
  (bind _wave (`self.Wave`))
  (if (`self.bWaveActive`)
    (bind _outactors (`GameplayStatics.GetAllActorsOfClass` "/Game/Bleuprints/BP_Enemy.BP_Enemy_C"))
    (if (< (`self.EnemiesSpawned`) (`self.EnemiesToSpawn`))
      (`self.SpawnEnemy`)
      (elif (== (`KismetArrayLibrary.Array_Length` _outactors) 0)
        (set `self.bWaveActive` false)
        (`KismetSystemLibrary.PrintString` "Oleada terminada")
        (if (== _wave (`self.WaveToWin`))
          (`|SpawnActorFromClass` "/Game/Bleuprints/BP_Boss.BP_Boss_C" (`KismetMathLibrary.MakeTransform` (+ (`self.K2_GetActorLocation`) (0.0 0.0 200.0))) "AdjustIfPossibleButAlwaysSpawn" "MultiplyWithRoot" null _wave null)
          (else
            (`KismetSystemLibrary.K2_SetTimerDelegate` (delegate `StartWave`) (`self.TimeBetweenWaves`))))))))

(event `self.ReceiveBeginPlay`
  (`KismetSystemLibrary.K2_SetTimerDelegate` (delegate `WaveTick`) (`self.SpawnIntertval`) true)
  (`KismetSystemLibrary.K2_SetTimerDelegate` (delegate `StartWave`) 3.0))

(fn `UserConstructionScript`)