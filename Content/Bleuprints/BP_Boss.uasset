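; Boss enemy "Guardian" that chases the player, shows a health bar and triggers the player's Victory on death.
; Looping timers drive movement and attacks, paused during slams: aimed bolt spreads, plus a flash-telegraphed radial slam with knock-up from phase two.
; Damage flashes the dynamic material, updates the bar and advances health-threshold phases announced on the player HUD.
; The final phase increases bolt count, changes walk speed and summons swarmers.
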(event `self.ReceiveBeginPlay`
  (bind _returnvalue (`PrimitiveComponent.CreateDynamicMaterialInstance` (`self.Body`) 0 null "None"))
  (set `self.HitMat` _returnvalue)
  (set `self.health` (`self.MaxHealth`))
  (bind _returnvalue_2 (`|CreateWidget` "/Game/Widgets/WBD_BossBar.WBD_BossBar_C" (`GameplayStatics.GetPlayerController` 0)))
  (bind _output_get (set `self.BarRef` _returnvalue_2))
  (`UserWidget.AddToViewport` _output_get 0)
  (`/Game/Widgets/WBD_BossBar.UpdateBar` (`self.BarRef`) (`self.health`) (`self.MaxHealth`))
  (`KismetSystemLibrary.K2_SetTimerDelegate` (delegate `Chase`) 0.3 true)
  (`KismetSystemLibrary.K2_SetTimerDelegate` (delegate `BossAttack`) 3.0 true))

(event `BossAttack`
  (if (and (not (`self.bIsDead`)) (not (`self.bBusy`)))
    (if (== (`self.Phase`) 1)
      (`self.ShootSpread`)
      (elif (`KismetMathLibrary.RandomBoolWithWeight` 0.5)
        (`self.Slam`)
        (else
          (`self.ShootSpread`))))))

(event `Chase`
  (if (and (not (`self.bIsDead`)) (not (`self.bBusy`)))
    (`|AIMoveTo` self (0.0 0.0 0.0) (`GameplayStatics.GetPlayerCharacter` 0) 250.0)))

(event `self.ReceiveAnyDamage`
  (params (Damage :type "Float (single-precision)") (DamageType :type "DamageType Object Reference") (InstigatedBy :type "Controller Object Reference") (DamageCauser :type "Actor Object Reference"))
  (if (not (`self.bIsDead`))
    (set `self.health` (`KismetMathLibrary.FClamp` (- (`self.health`) Damage) 0.0 (`self.MaxHealth`)))
    (`|ExecutionSequence`
      (:`then_0`
        (bind (_direction _flash) (`Timeline|HitTimeline` :!via `PlayFromStart`)
          (:`Update`
            (`MaterialInstanceDynamic.SetScalarParameterValue` (`self.HitMat`) "HitFlash" _flash))))
      (:`then_1`
        (`/Game/Widgets/WBD_BossBar.UpdateBar` (`self.BarRef`) (`self.health`) (`self.MaxHealth`))
        (`self.UpdatePhase`)
        (if (<= (`self.health`) 0.0)
          (`self.DIE`))))))

(event `UpdatePhase`
  (if (and (<= (/ (`self.health`) (`self.MaxHealth`)) 0.3) (< (`self.Phase`) 3))
    (set `self.Phase` 3)
    (`self.AnnouncePhase` "¿El Guardian se enfurece!")
    (set `CharacterMovementComponent.MaxWalkSpeed` 420.0 (`self.CharacterMovement`))
    (`self.SummonSwarm`)
    (elif (and (<= (/ (`self.health`) (`self.MaxHealth`)) 0.6) (< (`self.Phase`) 2))
      (set `self.Phase` 2)
      (`self.AnnouncePhase` "¿El Guardian golpea el sueelo!"))))

(event `DIE`
  (set `self.bIsDead` true)
  (`/Engine/EditorBlueprintResources/StandardMacros.IsValid` (`self.BarRef`)
    (:`Is Valid`
      (`Widget.RemoveFromParent` (`self.BarRef`)))
    (:`Is Not Valid`
      _))
  (`NiagaraFunctionLibrary.SpawnSystemAtLocation` "/Game/FX/NS_Explosion.NS_Explosion" (`self.K2_GetActorLocation`) (struct) (3.0 3.0 3.0))
  (bind _asbp_slime (cast `/Game/ThirdPerson/Blueprints/BP_Slime` (`GameplayStatics.GetPlayerCharacter` 0)))
  (`/Game/ThirdPerson/Blueprints/BP_Slime.Victory` _asbp_slime (`self.WavesCleared`))
  (`KismetSystemLibrary.Delay` 1.5)
  (`self.K2_DestroyActor`))

(event `AnnouncePhase`
  (params (Message :type Text))
  (bind _asbp_slime (cast `/Game/ThirdPerson/Blueprints/BP_Slime` (`GameplayStatics.GetPlayerCharacter` 0)))
  (bind _hudref (`/Game/ThirdPerson/Blueprints/BP_Slime.HUDRef` _asbp_slime))
  (`/Engine/EditorBlueprintResources/StandardMacros.IsValid` _hudref
    (:`Is Valid`
      (`/Game/Widgets/WBP_HUD.ShowUnlock` _hudref Message))))

(event `ShootSpread`
  (if (== (`self.Phase`) 3)
    (for _index (range 5)
      (`self.FireBolt` (* (- _index 2.0) 15.0)))
    (else
      (for _index_2 (range 1 4)
        (`self.FireBolt` (* (- _index_2 2.0) 15.0))))))

(event `Slam`
  (set `self.bBusy` true)
  (`MovementComponent.StopMovementImmediately` (`self.CharacterMovement`))
  (`MaterialInstanceDynamic.SetScalarParameterValue` (`self.HitMat`) "HitFlash" 1.0)
  (`KismetSystemLibrary.Delay` 1.0)
  (`MaterialInstanceDynamic.SetScalarParameterValue` (`self.HitMat`) "HitFlash" 0.0)
  (`NiagaraFunctionLibrary.SpawnSystemAtLocation` "/Game/FX/NS_Explosion.NS_Explosion" (`self.K2_GetActorLocation`) (struct) (1.5 1.5 1.5))
  (if (and (<= (`self.GetDistanceTo` (`GameplayStatics.GetPlayerCharacter` 0)) (`self.SlamRadius`)) (not (`self.bIsDead`)))
    (`GameplayStatics.ApplyDamage` (`GameplayStatics.GetPlayerCharacter` 0) (`self.SlamDamage`) null self)
    (`self.LaunchCharacter` (`GameplayStatics.GetPlayerCharacter` 0) (0.0 0.0 700.0) false true))
  (`KismetSystemLibrary.Delay` 0.6)
  (set `self.bBusy` false))

(event `SummonSwarm`
  (for _index (range 4)
    (`|SpawnActorFromClass` "/Game/Bleuprints/BP_Enemy.BP_Enemy_C" (`KismetMathLibrary.MakeTransform` (+ (`self.K2_GetActorLocation`) (`KismetMathLibrary.MakeVector` (- (* _index 250.0) 375.0) 300.0 80.0))) "AdjustIfPossibleButAlwaysSpawn" "MultiplyWithRoot" null (`self.SwarmerData`) null)))

(event `FireBolt`
  (params (Yaw :type "Float (double-precision)"))
  (bind _returnvalue (`KismetMathLibrary.ComposeRotators` (`KismetMathLibrary.FindLookAtRotation` (`self.K2_GetActorLocation`) (`self.K2_GetActorLocation` (`GameplayStatics.GetPlayerCharacter` 0))) (`KismetMathLibrary.MakeRotator` 0.0 0.0 Yaw)))
  (`|SpawnActorFromClass` "/Game/Bleuprints/BP_EnemyProjectile.BP_EnemyProjectile_C" (`KismetMathLibrary.MakeTransform` (+ (* (`KismetMathLibrary.GetForwardVector` _returnvalue) 250.0) (`self.K2_GetActorLocation`)) _returnvalue) "AlwaysSpawn" "MultiplyWithRoot" null (`self.ProjectileDamage`) null self))

(fn `UserConstructionScript`)