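; Enemy character configured by an EnemyData asset for stats and loot, plus mesh, scale and material applied in the construction script.
; Looping timers make it chase the player within aggro range and apply damage within attack range.
; Damage reduces health and plays a timeline-driven HitFlash on a dynamic material.
; The timeline update triggers death at zero health, spawning a BP_Absorbable with the loot data before destroying the enemy.
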(event `self.ReceiveBeginPlay`
  (bind _returnvalue (`PrimitiveComponent.CreateDynamicMaterialInstance` (`self.Cone`) 0 null "None"))
  (set `self.HitMat` _returnvalue)
  (`/Engine/EditorBlueprintResources/StandardMacros.IsValid` (`self.EnemyData`)
    (:`Is Valid`
      (set `self.MaxHealth` (`/Game/Bleuprints/DATAS/PDA_EnemyData.MaxHealth` (`self.EnemyData`)))
      (set `self.Health` (`/Game/Bleuprints/DATAS/PDA_EnemyData.MaxHealth` (`self.EnemyData`)))
      (set `CharacterMovementComponent.MaxWalkSpeed` (`/Game/Bleuprints/DATAS/PDA_EnemyData.MoveSpeed` (`self.EnemyData`)) (`self.CharacterMovement`))
      (set `self.AttackDamage` (`/Game/Bleuprints/DATAS/PDA_EnemyData.Damage` (`self.EnemyData`)))
      (set `self.AttackRange` (`/Game/Bleuprints/DATAS/PDA_EnemyData.AttackRange` (`self.EnemyData`)))
      (set `self.AggroRange` (`/Game/Bleuprints/DATAS/PDA_EnemyData.AggroRange` (`self.EnemyData`)))
      (set `self.LootData` (`/Game/Bleuprints/DATAS/PDA_EnemyData.LootData` (`self.EnemyData`))))
    (:`Is Not Valid`
      _))
  (`KismetSystemLibrary.K2_SetTimerDelegate` (delegate `Chase`) 0.3 true)
  (`KismetSystemLibrary.K2_SetTimerDelegate` (delegate `TryAttack`) (`KismetMathLibrary.SelectFloat` (`/Game/Bleuprints/DATAS/PDA_EnemyData.AttackInterval` (`self.EnemyData`)) 1.0 true) true))

(event `Chase`
  (if (< (`self.GetDistanceTo` (`GameplayStatics.GetPlayerCharacter` 0)) (`self.AggroRange`))
    (`|AIMoveTo` self (0.0 0.0 0.0) (`GameplayStatics.GetPlayerCharacter` 0) 120.0)))

(event `TryAttack`
  (if (<= (`self.GetDistanceTo` (`GameplayStatics.GetPlayerCharacter` 0)) (`self.AttackRange`))
    (`GameplayStatics.ApplyDamage` (`GameplayStatics.GetPlayerCharacter` 0) (`self.AttackDamage`) null self)))

(event `self.ReceiveAnyDamage`
  (params (Damage :type "Float (single-precision)") (DamageType :type "DamageType Object Reference") (InstigatedBy :type "Controller Object Reference") (DamageCauser :type "Actor Object Reference"))
  (if (not (`self.bIsDead`))
    (set `self.Health` (`KismetMathLibrary.FClamp` (- (`self.Health`) Damage) 0.0 (`self.MaxHealth`)))
    (bind (_direction _flash) (`Timeline|HitTimeline` :!via `PlayFromStart`)
      (:`Update`
        (`MaterialInstanceDynamic.SetScalarParameterValue` (`self.HitMat`) "HitFlash" _flash)
        (if (<= (`self.Health`) 0.0)
          (`self.Die`))))))

(event `Die`
  (set `self.bIsDead` true)
  (`/Engine/EditorBlueprintResources/StandardMacros.IsValid` (`self.LootData`)
    (:`Is Valid`
      (`|SpawnActorFromClass` "/Game/Bleuprints/BP_Absorbable.BP_Absorbable_C" (`KismetMathLibrary.MakeTransform` (+ (`self.K2_GetActorLocation`) (0.0 0.0 70.0))) "AlwaysSpawn" "MultiplyWithRoot" null (`self.LootData`) null))
    (:`Is Not Valid`
      _))
  (`self.K2_DestroyActor`))

(fn `UserConstructionScript`
  (`/Engine/EditorBlueprintResources/StandardMacros.IsValid` (`self.EnemyData`)
    (:`Is Valid`
      (`StaticMeshComponent.SetStaticMesh` (`self.Cone`) (`/Game/Bleuprints/DATAS/PDA_EnemyData.Mesh` (`self.EnemyData`)))
      (`SceneComponent.SetRelativeScale3D` (`self.Cone`) (`/Game/Bleuprints/DATAS/PDA_EnemyData.MeshScale` (`self.EnemyData`)))
      (`PrimitiveComponent.SetMaterial` (`self.Cone`) 0 (`/Game/Bleuprints/DATAS/PDA_EnemyData.Material` (`self.EnemyData`))))))