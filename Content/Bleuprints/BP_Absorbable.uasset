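; Absorbable object that BP_Slime can swallow and digest, with mesh, scale, material and mass set from its Data in the construction script.
; StartAbsorb disables physics and collision, then a timeline pulls it to the slime's AbsorbPoint while shrinking, and attaches it.
; A digestion timeline, restarted on every pull update and after attachment, shrinks it to zero at a Data-driven rate.
; It then grants nutrients, healing, stomach storage and a timed ability before destroying itself.
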(event `StartAbsorb`
  (params (Absorber :type "Actor Object Reference"))
  (bind _data (`self.Data`))
  (if (not (`self.IsAbsorbed`))
    (set `self.IsAbsorbed` true)
    (set `self.TargetActor` Absorber)
    (set `self.StartLocation` (`self.K2_GetActorLocation`))
    (set `self.OriginalScale` (`self.GetActorScale3D`))
    (`PrimitiveComponent.SetSimulatePhysics` (`self.Cube`) false)
    (`PrimitiveComponent.SetCollisionEnabled` (`self.Cube`) "NoCollision")
    (`GameplayStatics.PlaySoundAtLocation` "/Game/Audio/EatingSound.EatingSound" (`self.K2_GetActorLocation`) (struct) 1.0 (`KismetMathLibrary.RandomFloatInRange` 0.9 1.1) 0.0 null null null null)
    (`NiagaraFunctionLibrary.SpawnSystemAtLocation` null (`self.K2_GetActorLocation`))
    (bind (_direction _alpha) (`Timeline|AbsorbTimeline` :!via `PlayFromStart`)
      (:`Update`
        (`self.K2_SetActorLocation` (`KismetMathLibrary.VLerp` (`self.StartLocation`) (`SceneComponent.K2_GetComponentLocation` (`/Game/ThirdPerson/Blueprints/BP_Slime.AbsorbPoint` (cast `/Game/ThirdPerson/Blueprints/BP_Slime` (`self.TargetActor`) :!pure true))) _alpha))
        (`self.SetActorScale3D` (* (`self.OriginalScale`) (`KismetMathLibrary.Lerp` 1.0 0.3 _alpha))))
      (:`Finished`
        (`self.K2_AttachToActor` (`self.TargetActor`) "None" "KeepWorld" "KeepWorld" "KeepWorld" false)))
    (set `self.DigestStartScale` (`self.GetActorScale3D`))
    (`TimelineComponent.SetPlayRate` (`self.DigestionTimeline`) (/ 5.0 (`/Game/Bleuprints/DATAS/PDA_AbsotbableData.DigestSeconds` (`self.Data`))))
    (bind (_direction_2 _alpha_2) (`Timeline|DigestionTimeline` :!via `PlayFromStart`)
      (:`Update`
        (`self.SetActorScale3D` (`KismetMathLibrary.VLerp` (`self.DigestStartScale`) (0.0 0.0 0.0) _alpha_2)))
      (:`Finished`
        (bind _asbp_slime (cast `/Game/ThirdPerson/Blueprints/BP_Slime` (`self.TargetActor`)))
        (`/Game/ThirdPerson/Blueprints/BP_Slime.AddNutrients` _asbp_slime (`/Game/Bleuprints/DATAS/PDA_AbsotbableData.Nutrients` (`self.Data`)))
        (`/Game/ThirdPerson/Blueprints/BP_Slime.Heal` _asbp_slime (`/Game/Bleuprints/DATAS/PDA_AbsotbableData.HealAmount` (`self.Data`)))
        (`/Game/ThirdPerson/Blueprints/BP_Slime.StoreInStomach` _asbp_slime (`self.Data`))
        (`/Game/ThirdPerson/Blueprints/BP_Slime.GrantAbility` _asbp_slime (`/Game/Bleuprints/DATAS/PDA_AbsotbableData.Ability` _data) (`/Game/Bleuprints/DATAS/PDA_AbsotbableData.AbilityDuration` _data))
        (`self.K2_DestroyActor`)))))

(fn `UserConstructionScript`
  (`/Engine/EditorBlueprintResources/StandardMacros.IsValid` (`self.Data`)
    (:`Is Valid`
      (`StaticMeshComponent.SetStaticMesh` (`self.Cube`) (`/Game/Bleuprints/DATAS/PDA_AbsotbableData.Mesh` (`self.Data`)))
      (`SceneComponent.SetRelativeScale3D` (`self.Cube`) (`/Game/Bleuprints/DATAS/PDA_AbsotbableData.MeshScale` (`self.Data`)))
      (`PrimitiveComponent.SetMaterial` (`self.Cube`) 0 (`/Game/Bleuprints/DATAS/PDA_AbsotbableData.Material` (`self.Data`)))
      (`PrimitiveComponent.SetMassOverrideInKg` (`self.Cube`) "None" (`/Game/Bleuprints/DATAS/PDA_AbsotbableData.MassKg` (`self.Data`)) true))))